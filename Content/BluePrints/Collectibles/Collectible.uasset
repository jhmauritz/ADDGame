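; Collectible coin pickup that spins and adds to the player's coin count when touched.
; BeginPlay caches the player's ThirdPersonCharacter, and Tick rolls the Cylinder by YawPerSeconds scaled by delta time, despite the variable's yaw name.
; When the Cylinder overlaps that player, it increments Coins on the mygi GameInstance and destroys itself.
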(event `self.ReceiveBeginPlay`
  (bind _asthird_person_character (cast `/Game/BluePrints/Player/ThirdPersonCharacter` (`GameplayStatics.GetPlayerCharacter` 0)))
  (set `self.pLAYER` _asthird_person_character))

(event `self.ReceiveTick`
  (params (DeltaSeconds :type "Float (single-precision)"))
  (`SceneComponent.K2_AddLocalRotation` (`self.Cylinder`) (`KismetMathLibrary.MakeRotator` (* DeltaSeconds (`self.YawPerSeconds`))) false false))

(event `self.Cylinder.OnComponentBeginOverlap`
  (params (OverlappedComponent :type "PrimitiveComponent Object Reference") (OtherActor :type "Actor Object Reference") (OtherComp :type "PrimitiveComponent Object Reference") (OtherBodyIndex :type Integer) (bFromSweep :type Boolean) (SweepResult :type "HitResult Structure (by ref)"))
  (if (== OtherActor (`self.pLAYER`))
    (bind _asmygi (cast `/Game/BluePrints/Player/mygi` (`GameplayStatics.GetGameInstance`)))
    (set `/Game/BluePrints/Player/mygi.Coins` (+ (`/Game/BluePrints/Player/mygi.Coins` _asmygi) 1) _asmygi)
    (`self.K2_DestroyActor`)))

(fn `UserConstructionScript`)