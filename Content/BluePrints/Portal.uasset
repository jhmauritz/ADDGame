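; Portal actor that toggles the player between a hub and a level when the character enters its trigger.
; A UsedPortal flag picks the destination, updates the teleport flag on the mygi game instance, and plays an objective sound on entering the level.
; Tick moves the portal itself between its starting and new location markers to match that flag.
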(event `self.ReceiveActorBeginOverlap`
  (params (OtherActor :type "Actor Object Reference")))

(event `self.Trigger.OnComponentBeginOverlap`
  (params (OverlappedComponent :type "PrimitiveComponent Object Reference") (OtherActor :type "Actor Object Reference") (OtherComp :type "PrimitiveComponent Object Reference") (OtherBodyIndex :type Integer) (bFromSweep :type Boolean) (SweepResult :type "HitResult Structure (by ref)"))
  (bind _asthird_person_character (cast `/Game/BluePrints/Player/ThirdPersonCharacter` OtherActor))
  (bind _asmygi (cast `/Game/BluePrints/Player/mygi` (`GameplayStatics.GetGameInstance`)))
  (if (`self.UsedPortal`)
    (`self.K2_TeleportTo` :`self` _asthird_person_character :`DestLocation` (`self.K2_GetActorLocation` (`self.PlayerHubLoc`)))
    (set `/Game/BluePrints/Player/mygi.DidPLayerTeleport?` false _asmygi)
    (set `self.UsedPortal` false)
    (else
      (`self.K2_TeleportTo` :`self` _asthird_person_character :`DestLocation` (`self.K2_GetActorLocation` (`self.PlayerLevelLoc`)))
      (set `/Game/BluePrints/Player/mygi.DidPLayerTeleport?` true _asmygi)
      (`/Game/BluePrints/Player/mygi.PlaySoundForObjective` _asmygi)
      (set `self.UsedPortal` true))))

(event `self.ReceiveTick`
  (params (DeltaSeconds :type "Float (single-precision)"))
  (bind _startingposition (`self.StartingPosition`))
  (bind _portalnewlocation (`self.PortalNewLocation`))
  (`|ExecutionSequence`
    (:`then_0`
      (if (`self.UsedPortal`)
        (if (not (== (`self.K2_GetActorLocation` _portalnewlocation) (`self.K2_GetActorLocation`)))
          (`self.K2_TeleportTo` (`self.K2_GetActorLocation` _portalnewlocation) (`self.K2_GetActorRotation` _portalnewlocation)))
        (elif (not (== (`self.K2_GetActorLocation`) (`self.K2_GetActorLocation` (`self.StartingPosition`))))
          (`self.K2_TeleportTo` (`self.K2_GetActorLocation` _startingposition) (`self.K2_GetActorRotation` _startingposition)))))))

(fn `UserConstructionScript`)