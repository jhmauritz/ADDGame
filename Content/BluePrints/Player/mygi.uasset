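; Game Instance that persists coins, day and remaining level names through a single save slot and handles random level progression.
; Init restores only the day from an existing save, while SaveGame writes all three values to a fresh save object.
; LoadLevel refills an empty level list from the master list or otherwise reloads the saved one, then shuffles it, opens the first, removes it and saves, avoiding repeats until refill.
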(event `self.ReceiveInit`
  (bind _returnvalue (`GameplayStatics.DoesSaveGameExist` (`self.SvaeGameSlot`)))
  (if _returnvalue
    (bind _savedgame (`self.LoadGame`))
    (set `self.Day` (`/Game/BluePrints/Player/SaveGameObject.DaySaved` _savedgame))))

(fn `LoadGame`
  (returns (SavedGame :type "/Game/BluePrints/Player/SaveGameObject Object Reference"))
  (bind _svaegameslot (`self.SvaeGameSlot`))
  (bind _returnvalue (`GameplayStatics.CreateSaveGameObject` "/Game/BluePrints/Player/SaveGameObject.SaveGameObject_C"))
  (cast `/Game/BluePrints/Player/SaveGameObject` _returnvalue)
  (bind _returnvalue_2 (`GameplayStatics.DoesSaveGameExist` _svaegameslot))
  (if _returnvalue_2
    (bind _returnvalue_3 (`GameplayStatics.LoadGameFromSlot` _svaegameslot))
    (bind _assave_game_object (cast `/Game/BluePrints/Player/SaveGameObject` _returnvalue_3)
      (:`then`
        (return _assave_game_object))
      (:`CastFailed`
        _)))
  (return null))

(fn `LoadLevel`
  (if (== (`KismetArrayLibrary.Array_Length` (`self.LevelName`)) 0)
    (set `self.LevelName` (`self.LevelNameMaster`))
    (else
      (bind _savedgame (`self.LoadGame`))
      (set `self.LevelName` (`/Game/BluePrints/Player/SaveGameObject.LevelNameSaved` _savedgame))))
  (`KismetArrayLibrary.Array_Shuffle` (`self.LevelName`))
  (`GameplayStatics.OpenLevel` (`|GetArrayItem` (`self.LevelName`)))
  (`KismetArrayLibrary.Array_Remove` (`self.LevelName`))
  (`self.SaveGame`))

(fn `SaveGame`
  (returns (Sucess :type Boolean))
  (bind _returnvalue (`GameplayStatics.CreateSaveGameObject` "/Game/BluePrints/Player/SaveGameObject.SaveGameObject_C"))
  (bind _assave_game_object (cast `/Game/BluePrints/Player/SaveGameObject` _returnvalue)
    (:`then`
      (set `/Game/BluePrints/Player/SaveGameObject.CoinsSaved` (`self.Coins`) _assave_game_object)
      (set `/Game/BluePrints/Player/SaveGameObject.DaySaved` (`self.Day`) _assave_game_object)
      (set `/Game/BluePrints/Player/SaveGameObject.LevelNameSaved` (`self.LevelName`) _assave_game_object)
      (`GameplayStatics.SaveGameToSlot` _assave_game_object (`self.SvaeGameSlot`))
      (return true))
    (:`CastFailed`
      (return false))))